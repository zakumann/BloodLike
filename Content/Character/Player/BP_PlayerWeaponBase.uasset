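; BP_PlayerWeaponBase is the player weapon base, showing the weapon as a Paper2D flipbook with a bobbing motion.
; On BeginPlay, a SceneCaptureComponent2D is restricted to that flipbook, and InitializeWeapon clears and hides it.
; WeaponBobbing plays a timeline while moving that nudges the flipbook along relative Y from its current position.
; Stopping halts the timeline in place, as the interpolation back to the saved WeaponPosition is unwired.
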(event `self.ReceiveBeginPlay`
  (`SceneCaptureComponent.ShowOnlyComponent` (`self.SceneCaptureComponent2D`) (`self.WeaponFlipbook`))
  (set `self.WeaponPosition` (`SceneComponent.RelativeLocation` (`self.WeaponFlipbook`))))

(event `/Game/Character/Interfaces/INT_PlayerWeapon.InitializeWeapon`
  (bind _weaponflipbook (`self.WeaponFlipbook`))
  (`PaperFlipbookComponent.SetFlipbook` _weaponflipbook null)
  (`SceneComponent.SetHiddenInGame` _weaponflipbook true false))

(event `WeaponBobbing`
  (params (bIsMoving :type Boolean) (DeltaTime :type "Float (double-precision)"))
  (bind _weaponflipbook (`self.WeaponFlipbook`))
  (bind (_relativelocation_x _relativelocation_y _relativelocation_z) (`KismetMathLibrary.BreakVector` (`SceneComponent.RelativeLocation` _weaponflipbook)))
  (if bIsMoving
    (bind (_direction _weaponbobtrack) (`Timeline|Weaponbobbing_Timeline` :!label _label)
      (:`Update`
        (`SceneComponent.K2_SetRelativeLocation` _weaponflipbook (`KismetMathLibrary.MakeVector` _relativelocation_x (`KismetMathLibrary.Lerp` (+ _relativelocation_y 0.2) (- _relativelocation_y 0.2) _weaponbobtrack) _relativelocation_z) false false)))
    (else
      (`|ExecutionSequence`
        (:`then_0`
          (goto _label :!via `Stop`))))))

(fn `UserConstructionScript`)