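; BP_Pistol is a weapon actor that handles the pistol's flipbook visuals and firing flash.
; InitializeWeapon equips it by setting the idle flipbook and unhiding the sprite component.
; ShootPistol triggers a brief point light flash, plays the fire flipbook, then returns to idle after a delay equal to that flipbook's length.
; It contains only presentation logic, with no Tick, damage or ammo handling.
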(event `/Game/Character/Interfaces/INT_PlayerWeapon.InitializeWeapon`
  ; Equip Weapon
  (`PaperFlipbookComponent.SetFlipbook` (`self.WeaponFlipbook`) (`self.IdlePistol`))
  (`SceneComponent.SetHiddenInGame` (`self.WeaponFlipbook`) false false))

(event `ShootPistol`
  (bind _weaponflipbook (`self.WeaponFlipbook`))
  ; PistolFireAnimation
  (`self.LightFlash`)
  (`PaperFlipbookComponent.SetFlipbook` _weaponflipbook (`self.FirePistol`))
  (`KismetSystemLibrary.Delay` (`PaperFlipbookComponent.GetFlipbookLength` _weaponflipbook))
  (`PaperFlipbookComponent.SetFlipbook` (`self.WeaponFlipbook`) (`self.IdlePistol`)))

(event `LightFlash`
  (bind _pointlight (`self.PointLight`))
  ; Light Flash
  (`SceneComponent.SetHiddenInGame` _pointlight false false)
  (`KismetSystemLibrary.Delay` 0.25)
  (`SceneComponent.SetHiddenInGame` _pointlight true false))

(fn `UserConstructionScript`
  (`parent.UserConstructionScript`))