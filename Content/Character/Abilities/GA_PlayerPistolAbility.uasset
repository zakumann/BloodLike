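; Gameplay ability for the player's pistol, firing the weapon and applying an effect to the character it hits.
; FireWeapon lazily caches the owning player and the BP_Pistol from its weapon child actor, then calls ShootPistol.
; A debug-drawn Visibility line trace runs from the first-person camera out to WeaponRange.
; A hit FPSPlayerCharacter receives the effect, with the player as attacker.
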(event `self.FireWeapon`
  (bind _playerpistolweaponcomponent (`self.PlayerPistolWeaponComponent`))
  ; Fire Pistol
  (`self.GetPlayer`)
  (`self.GetWeapon`)
  (`/Engine/EditorBlueprintResources/StandardMacros.IsValid` _playerpistolweaponcomponent
    (:`Is Valid`
      (`/Game/Character/Weapons/BP_Pistol.ShootPistol` _playerpistolweaponcomponent)
      (bind _actor (`self.GetLineTrace`))
      (bind _asfpsplayer_character (cast `FPSPlayerCharacter` _actor))
      (`self.ApplyEffect` (`self.Player`) _asfpsplayer_character))))

(fn `GetLineTrace`
  (returns (Actor :type "Actor Object Reference"))
  (bind _firstpersoncamera (`/Game/Character/Player/BP_PlayerCharacter.FirstPersonCamera` (`self.Player`)))
  (bind _returnvalue (`SceneComponent.K2_GetComponentLocation` _firstpersoncamera))
  (bind _outhit (`KismetSystemLibrary.LineTraceSingle` :`Start` _returnvalue :`End` (+ _returnvalue (* (`KismetMathLibrary.GetForwardVector` (`SceneComponent.K2_GetComponentRotation` _firstpersoncamera)) (`self.Weapon Range`))) :`TraceChannel` "TraceTypeQuery1" :`DrawDebugType` "ForDuration"))
  (bind (_bblockinghit _binitialoverlap _time _distance _location _impactpoint _normal _impactnormal _physmat _hitactor) (`GameplayStatics.BreakHitResult` _outhit))
  (`/Engine/EditorBlueprintResources/StandardMacros.IsValid` _hitactor
    (:`Is Valid`
      (return _hitactor))))

(fn `GetPlayer`
  (bind _returnvalue_owneractor (break `GameplayAbilityActorInfo` (`self.GetActorInfo`)))
  (`/Engine/EditorBlueprintResources/StandardMacros.IsValid` (`self.Player`)
    (:`Is Valid`
      _)
    (:`Is Not Valid`
      (bind _asbp_player_character (cast `/Game/Character/Player/BP_PlayerCharacter` _returnvalue_owneractor))
      (set `self.Player` _asbp_player_character)))
  (return))

(fn `GetWeapon`
  (`/Engine/EditorBlueprintResources/StandardMacros.IsValid` (`self.PlayerPistolWeaponComponent`)
    (:`Is Valid`
      _)
    (:`Is Not Valid`
      (bind _asbp_pistol (cast `/Game/Character/Weapons/BP_Pistol` (`ChildActorComponent.ChildActor` (`/Game/Character/Player/BP_PlayerCharacter.Weapon` (`self.Player`)))))
      (set `self.PlayerPistolWeaponComponent` _asbp_pistol)))
  (return))