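; BP_WeaponPickup is a weapon pickup that equips its configured weapon on the player and then destroys itself.
; A looping timer started at BeginPlay periodically yaws the actor to face the player camera, with a 90-degree offset, avoiding per-frame Tick work.
; Overlap with a BP_PlayerCharacter calls EquipWeapon with WeaponToAcquire; other actors are ignored.
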(event `self.ReceiveBeginPlay`
  (`KismetSystemLibrary.K2_SetTimerDelegate` (delegate `DirectToPlayer`) 0.15 true)
  (`self.DirectToPlayer`))

(event `DirectToPlayer`
  (bind (_returnvalue_roll _returnvalue_pitch _returnvalue_yaw) (`KismetMathLibrary.BreakRotator` (`KismetMathLibrary.FindLookAtRotation` (`SceneComponent.K2_GetComponentLocation` (`self.Weapon`)) (`PlayerCameraManager.GetCameraLocation` (`GameplayStatics.GetPlayerCameraManager` 0)))))
  (`self.K2_SetActorRotation` (`KismetMathLibrary.MakeRotator` 0.0 0.0 (- _returnvalue_yaw 90.0))))

(event `self.ReceiveTick`
  (params (DeltaSeconds :type "Float (single-precision)")))

(event `self.ReceiveActorBeginOverlap`
  (params (OtherActor :type "Actor Object Reference"))
  (bind _asbp_player_character (cast `/Game/Character/BP_PlayerCharacter` OtherActor))
  (`/Game/Character/BP_PlayerCharacter.EquipWeapon` _asbp_player_character (`self.WeaponToAcquire`))
  (`self.K2_DestroyActor`))

(fn `UserConstructionScript`)