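; Base retro-FPS enemy character drawn as a flipbook sprite that yaws to face the player camera and runs a behavior tree through its AI controller.
; A looping timer computes the player's angle and side relative to the enemy's facing, choosing one of eight directional walk or idle flipbooks.
; Damage briefly plays a hurt flipbook, pausing directional updates.
; Death disables capsule collision and plays dying, then dead; attack events only print.
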(event `self.ReceiveBeginPlay`
  (`|ExecutionSequence`
    (:`then_0`
      (`KismetSystemLibrary.K2_SetTimerDelegate` (delegate `DirectToPlayer`) 0.1 true)
      (`self.DirectToPlayer`))
    (:`then_1`
      (bind _asbp_retro_fpsenemy_ai (cast `/Game/Enemies/AI/BP_RetroFPSEnemyAI` (`self.GetController`)))
      (`AIController.RunBehaviorTree` _asbp_retro_fpsenemy_ai (`self.BehaviorTree`)))))

(event `DirectToPlayer`
  (`self.SpriteFacePlayer`
    (:`Out`
      (if (not (or (`self.bIsDead`) (`self.bPauseAngleCalculations`)))
        (`self.GetEnemyAngle`
          (:`Out`
            (`self.CheckIfWalking`
              (:`Out`
                (`self.CalculateFlipbook`)))))))))

(event `self.TakeDamage`
  (params (CueData :type "GameplayCueParameters Structure"))
  (bind _enemy (`self.Enemy`))
  (`parent.TakeDamage` CueData)
  (if (not (`self.bIsDead`))
    (set `self.bPauseAngleCalculations` true)
    (`PaperFlipbookComponent.SetFlipbook` _enemy (`self.Damaged`))
    (`KismetSystemLibrary.Delay` (`PaperFlipbookComponent.GetFlipbookLength` _enemy))
    (set `self.bPauseAngleCalculations` false)))

(event `self.Kill Character`
  (bind _enemy (`self.Enemy`))
  (`parent.Kill Character`)
  (set `self.bIsDead` true)
  (`PrimitiveComponent.SetCollisionEnabled` (`self.CapsuleComponent`) "NoCollision")
  (`PaperFlipbookComponent.SetFlipbook` _enemy (`self.Dying`))
  (`KismetSystemLibrary.Delay` (`PaperFlipbookComponent.GetFlipbookLength` _enemy))
  (`PaperFlipbookComponent.SetFlipbook` (`self.Enemy`) (`self.Dead`)))

(event `Melee Attack`
  (`KismetSystemLibrary.PrintString` "MeleeAttack"))

(event `Ranged Attack`
  (`KismetSystemLibrary.PrintString` "RangedAttack"))

(fn `SetFlipbook`
  (params (Walking :type "PaperFlipbook Object Reference") (Idle :type "PaperFlipbook Object Reference"))
  (bind _enemy (`self.Enemy`))
  (if (`self.bIsWalking`)
    (`PaperFlipbookComponent.SetFlipbook` _enemy Walking)
    (else
      (`PaperFlipbookComponent.SetFlipbook` _enemy Idle))))

(fn `UserConstructionScript`)